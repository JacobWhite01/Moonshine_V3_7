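; Gravity well projectile for the Overlord that stuns mechs caught in its detonation sphere.
; Overlapping anything other than an Overlord or another gravity projectile spawns the grav well particle and, after a short delay, triggers Effect.
; Effect stops movement, calls StunMech on overlapping BP_MechPlayer actors with health left, then destroys the projectile.
; The owner is stored, but the collision filter checks class rather than that reference.
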(event OnComponentBeginOverlap(CollisionSphere)
  (params (OverlappedComponent :type Primitive%20Component%20Object%20Reference) (OtherActor :type Actor%20Object%20Reference) (OtherComp :type Primitive%20Component%20Object%20Reference) (OtherBodyIndex :type Integer) (bFromSweep :type Boolean) (SweepResult :type Hit%20Result%20Structure%20%28by%20ref%29))
  ;[1 1 1] Check when an actor is hit
  (if (and (!= OtherActor (.AsBP%20Overlord%20Gravity%20Projectile (Utilities|Casting|CastToBP_OverlordGravityProjectile OtherActor))) (!= (.AsBP%20Overlord (Utilities|Casting|CastToBP_Overlord OtherActor)) OtherActor))
    (Effects|SpawnEmitteratLocation "/Game/Assets/Particles/Weapons/P_OverlordGravWell.P_OverlordGravWell" (Transformation|GetActorLocation) "0, 0, 0" "0.500000,0.500000,0.500000")
    (Utilities|FlowControl|Delay 0.2)
    (CallFunction|Effect)))

(event Custom|Setup%20Owner%20Actor
  (params (Owner :type Actor%20Object%20Reference))
  ;[1 1 1] Set which mech owns this one (For collision)
  (Variables|Default|SetOwnerActor Owner))

(fn ConstructionScript)

(fn Effect
  ;[1 1 1] Stop projectile movement and begin checking all actors within detonation sphere
  (Components|Movement|StopMovementImmediately (Variables|Default|GetProjectileMovement))
  (for _array_element (Collision|GetOverlappingActors (Variables|Default|GetDetonation%20Sphere) "/Script/Engine.Actor" :!class /Script/Engine.PrimitiveComponent)
    (bind _asbp_mech_player (Utilities|Casting|CastToBP_MechPlayer _array_element))
    (bind _output_get (Variables|Default|SetHitMech _asbp_mech_player))
    (if (> (Variables|/Game/Blueprints/MechSide/BP_MechPlayer/BP_MechPlayer.BP_MechPlayer_C|GetHealth _output_get) 0.0)
      (Default|StunMech (Variables|Default|GetHitMech))))
  (Actor|DestroyActor))