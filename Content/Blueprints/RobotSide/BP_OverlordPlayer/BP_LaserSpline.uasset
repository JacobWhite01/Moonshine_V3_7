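; BP_LaserSpline is the visual laser beam for the Overlord player, drawn as a spline mesh between start and end locations.
; Tick refreshes the start from GetLaserStartPoint, whose Overlord firing-point lookup is left unused, while EndLocation is not set here.
; A looping timer lazily creates one spline mesh component and repeatedly stretches it between both locations, using tangents from the spline's points.
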(event Custom|Update%20Spline
  ;[1 1 1] Update all elements of spline mesh
  (for _index (range 0 (- (Spline|GetNumberOfSplinePoints (Variables|Default|GetSpline)) 2))
    ;[1 1 1] If the spline mesh has not been spawned, spawn it
    (if (Utilities|IsValid (Variables|Default|GetSplineMesh))
      _
      (else
        (bind _returnvalue (AddComponent|AddSplineMeshComponent true))
        (bind _output_get (Variables|Default|SetSplineMesh _returnvalue))))
    ;[1 1 1] Update Spline to Match start and end point of laser
    (SplineMesh|SetForwardAxis _output_get "X" true)
    (SplineMesh|SetStartandEnd (Variables|Default|GetSplineMesh) (Variables|Vectors|GetStart%20Location) (Spline|GetTangentatSplinePoint (Variables|Default|GetSpline) 0 "Local") (Variables|Vectors|GetEnd%20Location) (Spline|GetTangentatSplinePoint (Variables|Default|GetSpline) (+ _index 1) "Local") true :!class /Script/Engine.SplineMeshComponent)))

(event EventTick
  (params (DeltaSeconds :type Float%20%28single-precision%29))
  ;[1 1 1] Track Players Location
  (Variables|Vectors|SetStart%20Location (Utilities|GetLaserStartPoint)))

(event EventBeginPlay
  (Utilities|Time|SetTimerbyEvent (delegate Custom|Update%20Spline) 0.1 true))

(fn ConstructionScript)