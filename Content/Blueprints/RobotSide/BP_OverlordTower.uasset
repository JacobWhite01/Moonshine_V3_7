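; BP_OverlordTower is a robot-side defensive turret that attacks BP_MechPlayer actors entering its detection radius and is destroyed when its health runs out.
; The first detected mech becomes the target, the sphere rotates toward it each tick, and overlap starts a fire timer.
; Each shot line-traces from the eye, spawns a BP_TowerLaser and damages any mech hit.
; Retargeting takes the first overlapping mech, as the closest-distance check never runs.
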(event OnComponentEndOverlap(DetectionRadius)
  (params (OverlappedComponent :type Primitive%20Component%20Object%20Reference) (OtherActor :type Actor%20Object%20Reference) (OtherComp :type Primitive%20Component%20Object%20Reference) (OtherBodyIndex :type Integer))
  ;[1 1 1] Clear current target if it leaves detection radius
  (if (== (Variables|Targeting|GetCurrentTarget) OtherActor)
    (Variables|Targeting|SetCurrentTarget 0)))

(event OnComponentBeginOverlap(DetectionRadius)
  (params (OverlappedComponent :type Primitive%20Component%20Object%20Reference) (OtherActor :type Actor%20Object%20Reference) (OtherComp :type Primitive%20Component%20Object%20Reference) (OtherBodyIndex :type Integer) (bFromSweep :type Boolean) (SweepResult :type Hit%20Result%20Structure%20%28by%20ref%29))
  ;[1 0 0] Targeting
  ;;[1 1 1] When Overlapped, set variable for actor to attack unless the tower is dead
  (if (not (Variables|Health|GetIs%20Dead?))
    ;;[1 1 1] Attack targeted Minion
    (bind _asbp_mech_player (Utilities|Casting|CastToBP_MechPlayer OtherActor))
    ;;;[1 1 1] Set Targeted Actor
    (CallFunction|TargetDetectedActor _asbp_mech_player)
    (Utilities|Time|SetTimerbyEvent (delegate Custom|FireAtTargeted) (Variables|Firing|GetTurretFireRate) (Utilities|CheckifAnyTargetsRemain))))

(event Custom|FireAtTargeted
  ;[1 0 0] Targeting
  ;;[1 1 1] Attack targeted Minion
  (if (not (Variables|Health|GetIs%20Dead?))
    (Utilities|IsValid (Variables|Targeting|GetCurrentTarget)
      (:Is%20Valid
        (Firing|FireatTarget :!label _label))
      (:Is%20Not%20Valid
        (if (Utilities|CheckifAnyTargetsRemain)
          (Firing|GetClosestMech)
          (goto _label))))))

(event EventTick
  (params (DeltaSeconds :type Float%20%28single-precision%29))
  ;[1 1 1] Face Current Target
  (if (and (not (Variables|Health|GetIs%20Dead?)) (Utilities|IsValid (Variables|Targeting|GetCurrentTarget)))
    (Transformation|SetWorldRotation (Variables|Default|GetTowerSphere) (Utilities|FaceEnemyRotation) false false)))

(event Custom|TakeDamage
  (params (DamageAmount :type Float%20%28single-precision%29))
  ;[1 1 1] Take damage from Minion
  (bind _output_get (Variables|Health|SetHealth (- (Variables|Health|GetHealth) DamageAmount)))
  (if (<= _output_get 0.0)
    (Variables|Health|SetIs%20Dead? true)
    (Actor|DestroyActor)))

(fn ConstructionScript)

(fn GetClosestMech
  (bind _self self)
  (bind _detectionradius (Variables|Default|GetDetectionRadius))
  (bind _overlappingactors (Collision|GetOverlappingActors _detectionradius "/Game/Blueprints/MechSide/BP_MechPlayer/BP_MechPlayer.BP_MechPlayer_C" :!class /Script/Engine.PrimitiveComponent))
  (Variables|Targeting|SetClosest%20Target (Utilities|Array|Get(acopy) _overlappingactors))
  (for _array_element _overlappingactors
    (if (!= 0 0)
      (if (< (Transformation|GetDistanceTo _array_element _self) (Transformation|GetDistanceTo (Variables|Targeting|GetClosest%20Target) _self))
        (Variables|Targeting|SetClosest%20Target _array_element))))
  (Variables|Targeting|SetCurrentTarget (Variables|Targeting|GetClosest%20Target)))

(fn FireatTarget
  (bind _towereye (Variables|Default|GetTowerEye))
  ;[1 1 1] Trigger Line trace and use it spawn a tracer, to move towards the end position
  (bind _outhit (Collision|LineTraceByChannel (Transformation|GetWorldLocation (Variables|Default|GetTowerEye)) (Transformation|GetActorLocation (Variables|Targeting|GetCurrentTarget)) "TraceTypeQuery1" false 0 "ForOneFrame"))
  (bind _returnvalue (Game|SpawnActorfromClass "/Game/Blueprints/RobotSide/BP_TowerLaser.BP_TowerLaser_C" (Math|Transform|MakeTransform (Transformation|GetWorldLocation _towereye) (Transformation|GetWorldRotation _towereye)) "Undefined" 0 0))
  (bind _output_get (Variables|Default|SetSpawned%20Laser _returnvalue))
  (Variables|/Game/Blueprints/RobotSide/BP_TowerLaser.BP_TowerLaser_C|SetTower _output_get self)
  (Utilities|FlowControl|Sequence
    (:then_0
      ;[1 1 1] Deal Damage to mech
      (bind _asbp_mech_player (Utilities|Casting|CastToBP_MechPlayer (.HitActor (Collision|BreakHitResult _outhit))))
      (bind _output_get_2 (Variables|Default|SetHitActor _asbp_mech_player))
      (Variables|/Game/Blueprints/RobotSide/BP_TowerLaser.BP_TowerLaser_C|SetEnd%20Location (Variables|Default|GetSpawned%20Laser) (Transformation|GetActorLocation _output_get_2))
      (Default|TakeDamage _asbp_mech_player 25.0))
    (:then_1
      (return))))

(fn TargetDetectedActor
  (params (Actor :type Actor%20Object%20Reference))
  (if (not (Utilities|IsValid (Variables|Targeting|GetCurrentTarget)))
    (Variables|Targeting|SetCurrentTarget Actor)))