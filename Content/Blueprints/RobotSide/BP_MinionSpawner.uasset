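; BP_MinionSpawner spawns BP_MinionChar minions that are given lane objectives.
; On BeginPlay it stores the spawn points from CollectSpawns, then starts SpawnMinion, which re-calls itself after a fixed delay to produce endless waves.
; Each wave spawns one scaled minion per point and writes the first and second lane objectives into its Blackboard for the behavior tree.
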(event Custom|SpawnMinion
  ;[1 1 1] Spawn a Minion for every spawn point
  (for _array_element (Variables|Spawning|GetSpawnPointsLocal)
    (CallFunction|SpawnIndividualMinion _array_element))
  (Utilities|FlowControl|Delay 1e+01)
  (CallFunction|SpawnMinion))

(event Custom|SpawnIndividualMinion
  (params (SpawnPoint :type Scene%20Component%20Object%20Reference))
  ;[1 1 1] Spawn a Minion and assign its objective, passing it to a behaviour tree
  (bind _returnvalue (Game|SpawnActorfromClass "/Game/Blueprints/RobotSide/BP_Minions/BP_MinionChar.BP_MinionChar_C" (Math|Transform|MakeTransform (Transformation|GetWorldLocation SpawnPoint) "0, 0, 0" (Variables|Default|GetEnemyScale)) "Undefined" 0 0))
  (AI|Components|Blackboard|SetValueasObject (AI|GetBlackboard _returnvalue) (Utilities|String|StringToName "ObjectiveActor") (Variables|Default|GetLaneObjFirst))
  (AI|Components|Blackboard|SetValueasObject (AI|GetBlackboard _returnvalue) (Utilities|String|StringToName "SecondObjectiveActor") (Variables|Default|GetLaneObjSecond)))

(event EventBeginPlay
  ;[1 1 1] Get Spawn Points and Begin Spawning
  (Utilities|FlowControl|Sequence
    (:then_0
      (Variables|Spawning|SetSpawnPointsLocal (Utilities|CollectSpawns)))
    (:then_1
      (CallFunction|SpawnMinion))))

(fn ConstructionScript)