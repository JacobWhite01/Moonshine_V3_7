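; BP_MinionChar is a robot-side AI minion character that runs BP_MinionTree when possessed by its controller.
; Damage lowers health, plays a random impact sound and flags an attacking mech player in the blackboard, with retriggerable delays timing out both aggro and stun.
; Stuns zero walk speed, set StunnedBy and play a lift timeline.
; Death hides map markers, then spawns a particle burst and destroys the actor.
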(event EventPossessed
  (params (NewController :type Controller%20Object%20Reference))
  ;[1 1 1] Run Behaviour Tree when possessed
  (bind _asbp_minion_controller (Utilities|Casting|CastToBP_MinionController NewController))
  (AI|RunBehaviorTree _asbp_minion_controller "/Game/Blueprints/RobotSide/BP_Minions/Controllers/BP_MinionTree.BP_MinionTree"))

(event EventTick
  (params (DeltaSeconds :type Float%20%28single-precision%29))
  ;[1 1 1] Set visibility of health bar
  (if (not (and (Rendering|IsVisible (Variables|Default|GetHealthBar)) (> (Transformation|GetDistanceTo self (Game|GetPlayerCharacter 0)) 1e+02)))
    (Rendering|SetVisibility (Variables|Default|GetHealthBar) false false)))

(event EventBeginPlay
  ;[1 1 1] Reset rotation
  (Variables|Default|SetOriginalRotation (Transformation|GetActorRotation self)))

(event Custom|BeginDeathTimer
  ;[1 0 0] Death Process
  (Utilities|FlowControl|Sequence
    (:then_0
      ;;[1 1 1] Stop behaviour tree
      (bind _asbp_minion_controller (Utilities|Casting|CastToBP_MinionController (Pawn|GetController)))
      (AI|RunBehaviorTree _asbp_minion_controller)
      ;;[1 1 1] Set dead variable and hide map icon
      (Variables|Health|SetIsDead? true)
      (Rendering|SetVisibility (Variables|Default|GetMapSprite) false false))
    (:then_1
      ;;[1 1 1] Spawn emitter and destroy actor after duration
      (Utilities|FlowControl|Delay 0.5)
      (Effects|SpawnEmitteratLocation "/Game/Assets/ThirdParty/FXVarietyPack/Particles/P_ky_ThunderBallHit.P_ky_ThunderBallHit" (Transformation|GetWorldLocation (Variables|Default|GetMinionMesh)) "0, 0, 0" "2.000000,2.000000,2.000000")
      (Actor|DestroyActor))))

(event Custom|TakeDamage
  (params (DamageAmount :type Float%20%28single-precision%29) (Source :type Actor%20Object%20Reference))
  ;[1 0.2998 0] Take Damage
  (Variables|Health|SetDamage%20Source Source)
  (Utilities|FlowControl|Sequence
    (:then_0
      ;;[1 1 1] Select Random Impact Noise
      (Audio|SpawnSoundatLocation (Utilities|Select :Index (Math|Random|RandomInteger 1) :Option%200 "/Game/Sound/MinionImpact1.MinionImpact1" :Option%201 "/Game/Sound/MinionImpact2.MinionImpact2") (Transformation|GetActorLocation) "0, 0, 0" 1.0 1.0 0.0 0 0))
    (:then_1
      ;;[1 1 1] Take set externally set damage amount
      (bind _asbp_mech_player (Utilities|Casting|CastToBP_MechPlayer (Variables|Health|GetDamage%20Source))
        (:then
          (AI|Components|Blackboard|SetValueasObject (AI|GetBlackboard self) (Utilities|Name|MakeLiteralName "AttackingActor") _asbp_mech_player))
        (:CastFailed
          _))
      (Variables|Health|SetHealth (- (Variables|Health|GetHealth) DamageAmount))
      (Development|SetHiddeninGame (Variables|Default|GetAggroMarker) false false))
    (:then_2
      ;;[1 1 1] If attacked again continuing aggroing, stop after attacking ends
      (Utilities|FlowControl|RetriggerableDelay (Variables|Default|GetAggroTimer))
      (AI|Components|Blackboard|SetValueasObject (AI|GetBlackboard self) (Utilities|Name|MakeLiteralName "AttackingActor") 0)
      (Development|SetHiddeninGame (Variables|Default|GetAggroMarker) true false))))

(event Custom|StunMinion
  (params (Source :type Actor%20Object%20Reference) (Original%20Rotation :type Transform))
  ;[0 1 0.2617] Stun Minion
  (bind _output_get (Variables|Stunning|SetStunnedBy Source))
  (Utilities|FlowControl|Sequence
    (:then_0
      ;;[1 1 1] Set Actor stunned by
      (Variables|/Script/Engine.CharacterMovementComponent|SetMaxWalkSpeed (Variables|Character|GetCharacterMovement) 0.0)
      (AI|Components|Blackboard|SetValueasObject (AI|GetBlackboard self) (Utilities|Name|MakeLiteralName "StunnedBy") _output_get)
      (Variables|Default|SetCurrentLocation (Transformation|GetActorLocation))
      (bind _movementtrack (Timeline|LiftTimeline Play)
        (:Update
          (Transformation|SetActorLocation (Math|Vector|Lerp(Vector) (Variables|Default|GetCurrentLocation) (Math|Vector|MakeVector (.X (Math|Vector|BreakVector (Variables|Default|GetCurrentLocation))) (.Y (Math|Vector|BreakVector (Variables|Default|GetCurrentLocation))) (+ (.Z (Math|Vector|BreakVector (Variables|Default|GetCurrentLocation))) 1e+02)) _movementtrack) false false))
        (:Finished
          (CallFunction|ResetStunAnim))))
    (:then_1
      ;;[1 1 1] If stunned again continue being stunned, then resume normal activity
      (Utilities|FlowControl|RetriggerableDelay (Variables|Stunning|GetStunTimer))
      (Variables|/Script/Engine.CharacterMovementComponent|SetMaxWalkSpeed (Variables|Character|GetCharacterMovement) (Variables|Default|GetDefaultWalkSpeed))
      (AI|Components|Blackboard|SetValueasObject (AI|GetBlackboard self) (Utilities|Name|MakeLiteralName "StunnedBy") 0))))

(event Custom|ResetStunAnim
  (bind _currentlocation (Variables|Default|GetCurrentLocation))
  (bind (_x _y _z) (Math|Vector|BreakVector _currentlocation))
  ;[0 1 0.2617] Stun Minion
  (bind _movementtrack (Timeline|LiftTimeline SetNewTime)
    (:Update
      (Transformation|SetActorLocation (Math|Vector|Lerp(Vector) (Variables|Default|GetCurrentLocation) (Math|Vector|MakeVector _x _y (+ _z 1e+02)) _movementtrack) false false))
    (:Finished
      (CallFunction|ResetStunAnim))))

(fn ConstructionScript
  (Variables|/Script/Engine.CharacterMovementComponent|SetMaxWalkSpeed (Variables|Character|GetCharacterMovement) (Variables|Default|GetDefaultWalkSpeed)))