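; BP_DestructibleFence is an environment fence that breaks apart when damaged.
; Its Takedamage event accumulates damage, forwards each hit to the Destructible component with a fixed impulse strength, and disables the Box collision immediately.
; Once accumulated damage reaches DamageMax, a short delay precedes disabling collision on the Destructible itself.
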(event Custom|Take%20damage
  (params (Hit%20Location :type Vector) (ImpulseDir :type Vector%20%28by%20ref%29) (DamageAmount :type Float%20%28single-precision%29))
  (Variables|Default|SetDamage%20Taken (+ DamageAmount (Variables|Default|GetDamage%20Taken)))
  (Class|DestructibleComponent|ApplyDamage (Variables|Default|GetDestructible) DamageAmount Hit%20Location ImpulseDir 1e+02)
  (Collision|SetCollisionEnabled (Variables|Default|GetBox) "NoCollision")
  (if (>= (Variables|Default|GetDamage%20Taken) (Variables|Default|GetDamage%20Max))
    (Utilities|FlowControl|Delay 1.0)
    (Collision|SetCollisionEnabled (Variables|Default|GetDestructible) "NoCollision")))

(fn ConstructionScript)