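; BP_CableSpline is a spline-based cable actor that stores a power source and a power target.
; Its construction script tiles Z-forward spline mesh components along the spline in whole sections, with length scaled by the actor's Z scale.
; Each section takes its endpoints from the spline and clamps tangents to the section length.
; Destroyed events for the matching source or target only print debug messages.
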(event Custom|Power%20Source%20Destroyed?
  (params (Source :type Actor%20Object%20Reference))
  (if (== Source (Variables|Default|GetPower%20Source))
    (Development|PrintString "Source Destroyed!")))

(event Custom|Power%20Target%20Destroyed?
  (params (Target :type Actor%20Object%20Reference))
  (if (== Target (Variables|Default|GetPower%20Target))
    (Development|PrintString "Target Destroyed!")))

(fn ConstructionScript
  (bind _spline (Variables|Default|GetSpline))
  (bind _spline_2 (Variables|Default|GetSpline))
  ;[1 1 1] Update all elements of spline mesh
  (Variables|Default|SetSection%20Length (* (.z (Transformation|GetActorScale3D)) (Variables|Default|GetSection%20Length_Reference)))
  (for _index (range 0 (- (Math|Float|Truncate (/ (Spline|GetSplineLength (Variables|Default|GetSpline)) (Variables|Default|GetSection%20Length))) 1))
    ;[1 1 1] If the spline mesh has not been spawned, spawn it
    (bind _returnvalue (AddComponent|AddSplineMeshComponent false))
    ;[1 1 1] Update Spline start and end
    (SplineMesh|SetForwardAxis _returnvalue "Z" true)
    (SplineMesh|SetStartandEnd _returnvalue (Spline|GetLocationatDistanceAlongSpline _spline_2 (* _index (Variables|Default|GetSection%20Length)) "Local") (Math|Vector|ClampVectorSize (Spline|GetTangentatDistanceAlongSpline _spline_2 (* _index (Variables|Default|GetSection%20Length)) "Local") 0.0 (Variables|Default|GetSection%20Length)) (Spline|GetLocationatDistanceAlongSpline _spline (* (+ _index 1) (Variables|Default|GetSection%20Length)) "Local") (Math|Vector|ClampVectorSize (Spline|GetTangentatDistanceAlongSpline _spline (* (+ _index 1) (Variables|Default|GetSection%20Length)) "Local") 0.0 (Variables|Default|GetSection%20Length)) true :!class /Script/Engine.SplineMeshComponent)))