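; Hover component that pushes its owner's first primitive component, with physics enabled, away from surfaces below.
; Each tick it line-traces straight down and, on a hit, applies force from CalculateBounce and sets linear and angular damping.
; CalculateBounce contains an impact-normal force that fades with distance over the trace length, though that expression appears unconnected to any output.
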(event EventBeginPlay
  (bind _output_get (Variables|Default|SetPrimitiveComponent (Utilities|Array|Get(acopy) (Actor|GetComponentsByClass (Components|GetOwner) "/Script/Engine.PrimitiveComponent"))))
  (Physics|SetSimulatePhysics _output_get true))

(event EventTick
  (params (DeltaSeconds :type Float%20%28single-precision%29))
  (bind _returnvalue (Transformation|GetWorldLocation))
  (bind _primitivecomponent (Variables|Default|GetPrimitiveComponent))
  ;[1 1 1] Line Trace Directly Down
  (bind (_outhit _returnvalue_2) (Collision|LineTraceByChannel _returnvalue (- _returnvalue (Math|Vector|MakeVector 0.0 0.0 (Variables|Default|GetTraceLength))) "TraceTypeQuery1" true 0 "None"))
  (if _returnvalue_2
    (Physics|AddForce (Variables|Default|GetPrimitiveComponent) (Utilities|CalculateBounce (.Location (Collision|BreakHitResult _outhit)) (.ImpactNormal (Collision|BreakHitResult _outhit))) "None" false)
    (Class|PrimitiveComponent|SetLinearDamping _primitivecomponent (Variables|Default|GetLinDamp))
    (Class|PrimitiveComponent|SetAngularDamping _primitivecomponent (Variables|Default|GetAngDamp))))