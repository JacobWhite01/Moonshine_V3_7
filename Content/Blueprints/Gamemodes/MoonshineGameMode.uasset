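; Game mode for a local multiplayer match of mechs versus an Overlord, with a countdown ending in a paused leaderboard.
; BeginPlay creates players, pawns and per-player HUDs from tagged PlayerStarts, unless in footage mode.
; Deaths show a death camera and screen, then respawn after a delay: Overlord at its tagged start, mechs at a random PlayerController's location.
; Tick-driven Delay runs the timer; retriggerable delays clear three lane alerts.
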(event Custom|Spawn%20Death%20Camera%20%28Lord%29
  (params (Player%20Controller :type Player%20Controller%20Object%20Reference))
  ;[0 1 0.1003] Respawning
  ;;[1 1 1] Respawn Overlord
  (bind _returnvalue (Game|SpawnActorfromClass "/Game/Blueprints/BP_Components/BP_DeathCamera.BP_DeathCamera_C" (Variables|Death|GetDeathCameraTransform) "Undefined" 0 0))
  (Pawn|Possess Player%20Controller _returnvalue)
  (bind _returnvalue_2 (UserInterface|CreateWidget "/Game/UI/DeathScreens/BP_OverlordDeathScreen.BP_OverlordDeathScreen_C" Player%20Controller))
  (UserInterface|Viewport|AddtoPlayerScreen _returnvalue_2)
  (Utilities|FlowControl|Delay (Variables|Death|GetOverlordRespawnTime))
  (Widget|RemovefromParent _returnvalue_2)
  (bind _outactors (Actor|GetAllActorsOfClass "/Script/Engine.PlayerStart"))
  (for _array_element _outactors
    (if (Utilities|Name|Equal(Name) (Variables|/Script/Engine.PlayerStart|GetPlayerStartTag _array_element) "Overlord")
      (Spawning|RespawnOverlord _array_element Player%20Controller))))

(event Custom|Send%20Lane%20Alert
  (params (Lane :type Integer))
  (bind _lane_alerted (Variables|Default|GetLane%20Alerted))
  (bind _lane_alerted_2 (Variables|Default|GetLane%20Alerted))
  (bind _lane_alerted_3 (Variables|Default|GetLane%20Alerted))
  (bind _output (Utilities|Array|Get(acopy) _lane_alerted 2))
  (bind _output_2 (Utilities|Array|Get(acopy) _lane_alerted_2))
  (bind _output_3 (Utilities|Array|Get(acopy) _lane_alerted_3 1))
  ;[1 0.1427 0] Lane Alerts System
  (Utilities|FlowControl|Sequence
    (:then_0
      ;;[1 1 1] If Lane alert is for Lane 0, set it to be alerted and reset if not retriggered, after delay
      (if (== Lane 0)
        (Utilities|Array|SetArrayElem _lane_alerted_2 _output_2 1)
        (Utilities|FlowControl|RetriggerableDelay 3.0)
        (Utilities|Array|SetArrayElem _lane_alerted_2 _output_2 0)))
    (:then_1
      ;;[1 1 1] If Lane alert is for Lane 1, set it to be alerted and reset if not retriggered, after delay
      (if (== Lane 1)
        (Utilities|Array|SetArrayElem _lane_alerted_3 _output_3 1)
        (Utilities|FlowControl|RetriggerableDelay 3.0)
        (Utilities|Array|SetArrayElem _lane_alerted_3 _output_3 0)))
    (:then_2
      ;;[1 1 1] If Lane alert is for Lane 2, set it to be alerted and reset if not retriggered, after delay
      (if (== Lane 2)
        (Utilities|Array|SetArrayElem _lane_alerted _output 1)
        (Utilities|FlowControl|RetriggerableDelay 3.0)
        (Utilities|Array|SetArrayElem _lane_alerted _output 0)))))

(event Custom|Spawn%20Death%20Camera%20%28Mech%29
  (params (Player%20Controller :type Player%20Controller%20Object%20Reference))
  ;[0 1 0.1003] Respawning
  ;;[1 1 1] Respawn Mech
  (bind _returnvalue (Game|SpawnActorfromClass "/Game/Blueprints/BP_Components/BP_DeathCamera.BP_DeathCamera_C" (Variables|Death|GetDeathCameraTransform) "Undefined" 0 0))
  (Pawn|Possess Player%20Controller _returnvalue)
  (bind _returnvalue_2 (UserInterface|CreateWidget "/Game/UI/DeathScreens/BP_MechDeathScreen.BP_MechDeathScreen_C" Player%20Controller))
  (UserInterface|Viewport|AddtoPlayerScreen _returnvalue_2)
  (Utilities|FlowControl|Delay (Variables|Death|GetMechRespawnTime))
  (Widget|RemovefromParent _returnvalue_2)
  (bind _outactors (Actor|GetAllActorsOfClass "/Script/Engine.PlayerController"))
  (Spawning|RespawnMech (Utilities|Array|Get(acopy) _outactors (Math|Random|RandomIntegerinRange 0 2)) Player%20Controller))

(event EventBeginPlay
  ;[0.02881 1 0] Spawns 3 players
  (if (not (Variables|Default|GetIn%20footage%20mode?))
    (Utilities|FlowControl|Sequence
      (:then_0
        (Spawning|CreateMechs))
      (:then_1
        (Spawning|CreateOverlord))
      (:then_2
        (CallFunction|ResetPlayerStartTags))
      (:then_3
        ;[1 1 1] Disables all Player Input in menus
        (bind _outactors (Actor|GetAllActorsOfClass "/Script/Engine.PlayerController"))
        (for _array_element _outactors
          (Input|SetInputModeGameOnly _array_element))
        (Variables|/Script/Engine.PlayerController|SetbShowMouseCursor (Game|GetPlayerController 0) false)))))

(event EventTick
  (params (DeltaSeconds :type Float%20%28single-precision%29))
  ;[1 0 0] Timer counting down
  (Utilities|FlowControl|Delay 1.0)
  (CallFunction|RunTimer))

(fn ConstructionScript)

(fn SpawnOtherMechs
  (params (Spawn%20Point :type Actor%20Object%20Reference))
  (bind _asplayer_start (Utilities|Casting|CastToPlayerStart Spawn%20Point))
  (bind _playerstarttag (Variables|/Script/Engine.PlayerStart|GetPlayerStartTag _asplayer_start))
  (if (and (Utilities|Name|NotEqual(Name) _playerstarttag "Overlord") (Utilities|Name|NotEqual(Name) _playerstarttag "Used"))
    (bind _returnvalue (Class|GameplayStatics|CreatePlayer -1))
    (bind _returnvalue_2 (Game|SpawnActorfromClass "/Game/Blueprints/MechSide/BP_MechPlayer/BP_MechPlayer.BP_MechPlayer_C" (Math|Transform|MakeTransform (Transformation|GetActorLocation Spawn%20Point) (Transformation|GetActorRotation Spawn%20Point)) "Undefined" 0 0))
    (Pawn|Possess _returnvalue _returnvalue_2)
    (bind _returnvalue_3 (UserInterface|CreateWidget "/Game/UI/In-Game/BP_MechScreen.BP_MechScreen_C" _returnvalue))
    (Variables|/Game/Blueprints/MechSide/BP_MechPlayer/BP_MechPlayer.BP_MechPlayer_C|SetScreenWidget _returnvalue_2 _returnvalue_3)
    (UserInterface|Viewport|AddtoPlayerScreen _returnvalue_3)))

(fn SpawnFirstMech
  (params (Location :type Actor%20Object%20Reference))
  (bind _returnvalue (Game|GetPlayerController 0))
  (bind _returnvalue_2 (Game|SpawnActorfromClass "/Game/Blueprints/MechSide/BP_MechPlayer/BP_MechPlayer.BP_MechPlayer_C" (Math|Transform|MakeTransform (Transformation|GetActorLocation Location) (Transformation|GetActorRotation Location)) "Undefined" 0 0))
  (Pawn|Possess _returnvalue _returnvalue_2)
  (bind _returnvalue_3 (UserInterface|CreateWidget "/Game/UI/In-Game/BP_MechScreen.BP_MechScreen_C" _returnvalue))
  (Variables|/Game/Blueprints/MechSide/BP_MechPlayer/BP_MechPlayer.BP_MechPlayer_C|SetScreenWidget _returnvalue_2 _returnvalue_3)
  (UserInterface|Viewport|AddtoPlayerScreen _returnvalue_3))

(fn SpawnOverlord
  (params (Spawn%20Point :type Actor%20Object%20Reference))
  (if (Utilities|Name|Equal(Name) (Variables|/Script/Engine.PlayerStart|GetPlayerStartTag (.AsPlayer%20Start (Utilities|Casting|CastToPlayerStart Spawn%20Point))) "Overlord")
    (bind _returnvalue (Class|GameplayStatics|CreatePlayer -1))
    (bind _returnvalue_2 (Game|SpawnActorfromClass "/Game/Blueprints/RobotSide/BP_OverlordPlayer/BP_Overlord.BP_Overlord_C" (Math|Transform|MakeTransform (Transformation|GetActorLocation Spawn%20Point) (Transformation|GetActorRotation Spawn%20Point)) "Undefined" 0 0))
    (Pawn|Possess _returnvalue _returnvalue_2)
    (bind _returnvalue_3 (UserInterface|CreateWidget "/Game/UI/In-Game/BP_OverlordScreen.BP_OverlordScreen_C" _returnvalue))
    (Variables|/Game/Blueprints/RobotSide/BP_OverlordPlayer/BP_Overlord.BP_Overlord_C|SetHUD _returnvalue_2 _returnvalue_3)
    (UserInterface|Viewport|AddtoPlayerScreen _returnvalue_3)))

(fn CreateOverlord
  (bind _outactors (Actor|GetAllActorsOfClass "/Script/Engine.PlayerStart"))
  (for _array_element _outactors
    (Spawning|SpawnOverlord _array_element)))

(fn CreateMechs
  (bind _outactors (Actor|GetAllActorsOfClass "/Script/Engine.PlayerStart"))
  (Spawning|SpawnFirstMech (Utilities|Array|Get(acopy) _outactors))
  (Variables|/Script/Engine.PlayerStart|SetPlayerStartTag (Utilities|Array|Get(acopy) _outactors) "Used")
  (for _array_element _outactors
    (Spawning|SpawnOtherMechs _array_element)))

(fn ResetPlayerStartTags
  (bind _outactors (Actor|GetAllActorsOfClass "/Script/Engine.PlayerStart"))
  (for _array_element _outactors
    (if (Utilities|Name|NotEqual(Name) (Variables|/Script/Engine.PlayerStart|GetPlayerStartTag _array_element) "Overlord")
      (Variables|/Script/Engine.PlayerStart|SetPlayerStartTag _array_element "Mech"))))

(fn RunTimer
  (bind _returnvalue (Game|GetPlayerController 0))
  (Variables|Timer|SetSeconds (- (Variables|Timer|GetSeconds) 1))
  (if (< (Variables|Timer|GetSeconds) 0)
    (Variables|Timer|SetMinutes (- (Variables|Timer|GetMinutes) 1))
    (Variables|Timer|SetSeconds 59))
  (if (== (Variables|Timer|GetSeconds) 0)
    (if (== (Variables|Timer|GetMinutes) 0)
      (Viewport|RemoveAllWidgets)
      (bind _returnvalue_2 (UserInterface|CreateWidget "/Game/UI/BP_LeaderBoard.BP_LeaderBoard_C" _returnvalue))
      (UserInterface|Viewport|AddtoViewport _returnvalue_2 0)
      (Input|SetInputModeUIOnly _returnvalue _returnvalue_2 "DoNotLock")
      (Game|SetGamePaused true))))

(fn RespawnMech
  (params (Location :type Actor%20Object%20Reference) (Player%20Controller :type Player%20Controller%20Object%20Reference))
  (bind _returnvalue (Game|SpawnActorfromClass "/Game/Blueprints/MechSide/BP_MechPlayer/BP_MechPlayer.BP_MechPlayer_C" (Math|Transform|MakeTransform (Transformation|GetActorLocation Location) (Transformation|GetActorRotation Location)) "Undefined" 0 0))
  (Pawn|Possess Player%20Controller _returnvalue)
  (bind _returnvalue_2 (UserInterface|CreateWidget "/Game/UI/In-Game/BP_MechScreen.BP_MechScreen_C" Player%20Controller))
  (Variables|/Game/Blueprints/MechSide/BP_MechPlayer/BP_MechPlayer.BP_MechPlayer_C|SetScreenWidget _returnvalue _returnvalue_2)
  (UserInterface|Viewport|AddtoPlayerScreen _returnvalue_2))

(fn RespawnOverlord
  (params (Location :type Actor%20Object%20Reference) (Player%20Controller :type Player%20Controller%20Object%20Reference))
  (bind _returnvalue (Game|SpawnActorfromClass "/Game/Blueprints/RobotSide/BP_OverlordPlayer/BP_Overlord.BP_Overlord_C" (Math|Transform|MakeTransform (Transformation|GetActorLocation Location) (Transformation|GetActorRotation Location)) "Undefined" 0 0))
  (Pawn|Possess Player%20Controller _returnvalue)
  (bind _returnvalue_2 (UserInterface|CreateWidget "/Game/UI/In-Game/BP_OverlordScreen.BP_OverlordScreen_C" Player%20Controller))
  (Variables|/Game/Blueprints/RobotSide/BP_OverlordPlayer/BP_Overlord.BP_Overlord_C|SetHUD _returnvalue _returnvalue_2)
  (UserInterface|Viewport|AddtoPlayerScreen _returnvalue_2))