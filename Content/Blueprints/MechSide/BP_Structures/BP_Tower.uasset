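; BP_Tower is a lane defense turret that fires on minions and Overlords entering its detection radius.
; It faces its current target and uses timers to fire line traces with cosmetic tracers, ragdolling minions in one hit or damaging the Overlord.
; It retargets to the first overlapping minion, as the closest-distance check never runs.
; Taking damage alerts the game mode by lane, and death fractures a destructible before destroying the actor.
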(event OnComponentEndOverlap(DetectionRadius)
  (params (OverlappedComponent :type Primitive%20Component%20Object%20Reference) (OtherActor :type Actor%20Object%20Reference) (OtherComp :type Primitive%20Component%20Object%20Reference) (OtherBodyIndex :type Integer))
  ;[1 1 1] Clear current target if it leaves detection radius
  (if (== (Variables|Targeting|GetCurrentTarget) OtherActor)
    (Variables|Targeting|SetCurrentTarget 0)))

(event OnComponentBeginOverlap(DetectionRadius)
  (params (OverlappedComponent :type Primitive%20Component%20Object%20Reference) (OtherActor :type Actor%20Object%20Reference) (OtherComp :type Primitive%20Component%20Object%20Reference) (OtherBodyIndex :type Integer) (bFromSweep :type Boolean) (SweepResult :type Hit%20Result%20Structure%20%28by%20ref%29))
  ;[1 0 0] Targeting
  ;;[1 1 1] When Overlapped, set variable for actor to attack unless the tower is dead
  (if (not (Variables|Health|GetIs%20Dead?))
    (Utilities|FlowControl|Sequence
      (:then_0
        ;;[1 1 1] Attack targeted Minion
        (bind _asbp_minion_char (Utilities|Casting|CastToBP_MinionChar OtherActor))
        ;;;[1 1 1] Set Targeted Actor
        (CallFunction|TargetDetectedActor _asbp_minion_char)
        (Utilities|Time|SetTimerbyEvent (delegate Custom|FireAtTargeted) (Variables|Firing|GetTurretFireRate) (Utilities|CheckifAnyTargetsRemain)))
      (:then_1
        (bind _asbp_overlord (Utilities|Casting|CastToBP_Overlord OtherActor))
        (if (not (Utilities|IsValid (Variables|Targeting|GetCurrentTarget)))
          (CallFunction|TargetDetectedActor _asbp_overlord)
          (Utilities|Time|SetTimerbyEvent (delegate Custom|Attack%20Overlord) (Variables|Firing|GetTurretFireRate) (Utilities|CheckifAnyTargetsRemain)))))))

(event Custom|FireAtTargeted
  ;[1 0 0] Targeting
  ;;[1 1 1] Attack targeted Minion
  (if (not (Variables|Health|GetIs%20Dead?))
    (Utilities|IsValid (Variables|Targeting|GetCurrentTarget)
      (:Is%20Valid
        (Firing|FireatTarget :!label _label)
        (Utilities|FlowControl|Delay 0.1)
        (Components|Activation|Deactivate (Variables|Default|GetMuzzleFlare1)))
      (:Is%20Not%20Valid
        (if (Utilities|CheckifAnyTargetsRemain)
          (Firing|GetClosestMinion)
          (goto _label))))))

(event Custom|Attack%20Overlord
  ;[1 0 0] Targeting
  ;;[1 1 1] Fire at attacked actor until it is dead, then switch targets until none remain in range
  (if (not (Variables|Health|GetIs%20Dead?))
    (Utilities|IsValid (Variables|Targeting|GetCurrentTarget)
      (:Is%20Valid
        (Firing|FireatTarget)
        (Utilities|FlowControl|Delay 0.1 :!label _label)
        (Components|Activation|Deactivate (Variables|Default|GetMuzzleFlare)))
      (:Is%20Not%20Valid
        (if (Utilities|CheckifAnyTargetsRemain)
          (Firing|GetClosestMinion)
          (Firing|FireatTarget)
          (goto _label))))))

(event EventTick
  (params (DeltaSeconds :type Float%20%28single-precision%29))
  ;[1 1 1] Face Current Target
  (if (and (not (Variables|Health|GetIs%20Dead?)) (Utilities|IsValid (Variables|Targeting|GetCurrentTarget)))
    (Transformation|SetWorldRotation (Variables|Default|GetTurretPivot) (Utilities|FaceEnemyRotation) false false)))

(event Custom|TakeDamage
  (params (DamageAmount :type Float%20%28single-precision%29))
  ;[1 1 1] Take damage from Minion
  (Default|SendTowerAlert (Utilities|GetGamemode) (Variables|Default|GetLane))
  (bind _output_get (Variables|Health|SetHealth (- (Variables|Health|GetHealth) DamageAmount)))
  (if (<= _output_get 0.0)
    ;[1 1 1] Enable dead variable to prevent firing, disable and enable collision to prepare explosion
    (Variables|Health|SetIs%20Dead? true)
    (Collision|SetCollisionEnabled (Variables|Default|GetCollisionBox) "NoCollision")
    (Collision|SetCollisionEnabled (Variables|Default|GetTurretMesh) "QueryAndPhysics")
    (Class|DestructibleComponent|ApplyDamage (Variables|Default|GetDestructible) 1.0 (Transformation|GetWorldLocation (Variables|Default|GetDestructable%20Loc)) (Math|Vector|MakeVector 0.0 0.0 1e+02) 1e+02)
    (Physics|SetSimulatePhysics (Variables|Default|GetTurretMesh) true)
    (Utilities|FlowControl|Delay 4.0)
    (Actor|DestroyActor)))

(fn ConstructionScript)

(fn HitMinion
  (params (Hit :type Hit%20Result%20Structure%20%28by%20ref%29))
  (bind (_bblockinghit _binitialoverlap _time _distance _location _impactpoint _normal _impactnormal _physmat _hitactor) (Collision|BreakHitResult Hit))
  (bind (_impulse _location_2) (Utilities|CalculateImpact _impactpoint))
  ;[1 1 1] Kill Minion if Hit and apply impulse
  (bind _asbp_minion_char (Utilities|Casting|CastToBP_MinionChar _hitactor))
  (if (not (Variables|/Game/Blueprints/RobotSide/BP_Minions/BP_MinionChar.BP_MinionChar_C|GetIsDead? _asbp_minion_char))
    (Collision|SetCollisionEnabled (Variables|/Script/Engine.Character|GetCapsuleComponent _asbp_minion_char) "NoCollision")
    (Physics|SetSimulatePhysics (Variables|/Game/Blueprints/RobotSide/BP_Minions/BP_MinionChar.BP_MinionChar_C|GetMinionMesh _asbp_minion_char) true)
    (Physics|AddImpulseatLocation (Variables|/Game/Blueprints/RobotSide/BP_Minions/BP_MinionChar.BP_MinionChar_C|GetMinionMesh _asbp_minion_char) _impulse _location_2 "None")
    (Default|BeginDeathTimer _asbp_minion_char)
    (Firing|GetClosestMinion)))

(fn GetClosestMinion
  (bind _self self)
  (bind _detectionradius (Variables|Default|GetDetectionRadius))
  (bind _overlappingactors (Collision|GetOverlappingActors _detectionradius "/Game/Blueprints/RobotSide/BP_Minions/BP_MinionChar.BP_MinionChar_C" :!class /Script/Engine.PrimitiveComponent))
  (Variables|Targeting|SetClosest%20Target (Utilities|Array|Get(acopy) _overlappingactors))
  (for _array_element _overlappingactors
    (if (!= 0 0)
      (if (< (Transformation|GetDistanceTo _array_element _self) (Transformation|GetDistanceTo (Variables|Targeting|GetClosest%20Target) _self))
        (Variables|Targeting|SetClosest%20Target _array_element))))
  (Variables|Targeting|SetCurrentTarget (Variables|Targeting|GetClosest%20Target)))

(fn FireatTarget
  ;[1 1 1] Trigger Line trace and use it spawn a tracer, to move towards the end position
  (bind _outhit (Collision|LineTraceByChannel (Transformation|GetWorldLocation (Variables|Default|GetTurretBarrel)) (Transformation|GetActorLocation (Variables|Targeting|GetCurrentTarget)) "TraceTypeQuery1" false 0 "ForOneFrame"))
  (bind _returnvalue (Game|SpawnActorfromClass "/Game/Blueprints/MechSide/BP_Weapons/BP_Weapons/Projectiles/BP_ProjectileTracer.BP_ProjectileTracer_C" (Math|Transform|MakeTransform (Transformation|GetWorldLocation (Variables|Default|GetTurretBarrel)) (Transformation|GetWorldRotation (Variables|Default|GetTurretMesh))) "Undefined" 0 0))
  (Variables|/Game/Blueprints/MechSide/BP_Weapons/BP_Weapons/Projectiles/BP_ProjectileTracer.BP_ProjectileTracer_C|SetObjectiveLocation%20 _returnvalue (.TraceEnd (Collision|BreakHitResult _outhit)))
  (Utilities|FlowControl|Sequence
    (:then_0
      ;[1 1 1] Deal Damage to Minion
      (Utilities|Casting|CastToBP_MinionChar (.HitActor (Collision|BreakHitResult _outhit)))
      (Firing|HitMinion _outhit))
    (:then_1
      ;[1 1 1] Deal Damage to Overlord
      (bind _asbp_overlord (Utilities|Casting|CastToBP_Overlord (.HitActor (Collision|BreakHitResult _outhit))))
      (Default|TakeDamage _asbp_overlord (Variables|Firing|GetOverlordDamage)))
    (:then_2
      (return)))
  (Components|Activation|Activate (Variables|Default|GetMuzzleFlare) false))

(fn TargetDetectedActor
  (params (Actor :type Actor%20Object%20Reference))
  (if (not (Utilities|IsValid (Variables|Targeting|GetCurrentTarget)))
    (Variables|Targeting|SetCurrentTarget Actor)))