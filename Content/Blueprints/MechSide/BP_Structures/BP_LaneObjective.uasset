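; BP_LaneObjective is a destructible lane objective structure with a health pool.
; Its TakeDamage event subtracts incoming damage from Health.
; At zero or below, it applies damage with an upward impulse to its destructible mesh, then destroys the actor after a short delay.
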(event Custom|TakeDamage
  (params (DamageAmount :type Float%20%28single-precision%29))
  (bind _output_get (Variables|Default|SetHealth (- (Variables|Default|GetHealth) DamageAmount)))
  (if (<= _output_get 0.0)
    (Class|DestructibleComponent|ApplyDamage (Variables|Default|GetObjectiveDestructMesh) 1.0 (Transformation|GetWorldLocation (Variables|Default|GetObjectiveDestructMesh)) (Math|Vector|MakeVector 0.0 0.0 1e+02) 1e+02)
    (Utilities|FlowControl|Delay 4.0)
    (Actor|DestroyActor)))

(fn ConstructionScript)