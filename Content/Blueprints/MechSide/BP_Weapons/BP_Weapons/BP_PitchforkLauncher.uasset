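; BP_PitchforkLauncher is a charge-up mech weapon that launches pitchfork projectiles.
; Holding fire runs a looping timer that builds and debug-prints Charge, firing automatically at full charge or on release, with no minimum charge enforced.
; Each shot plays a camera shake and spawns a projectile at the barrel, aimed by camera rotation with velocity set from Charge.
; It then resets Charge and blocks firing and charging during a cooldown.
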(event Custom|Charge%20Weapon
  ;[0 1 0.162] Weapon Charging
  ;;[1 1 1] Charge weapon and fire if at 100%
  (if (not (Variables|Default|GetFired%20Recently?))
    (if (>= (Variables|Charge|GetCharge) 1e+02)
      (CallFunction|FireOnce)
      (else
        (bind _output_get (Variables|Charge|SetCharge (+ (Variables|Charge|GetCharge) (Variables|Charge|GetCharge%20Increment))))
        (Development|PrintString (Utilities|String|ToString(Float) _output_get))))))

(event Custom|Cancel%20Charging
  ;[0 1 0.162] Weapon Charging
  ;;[1 1 1] Cancel Charging
  (Utilities|Time|ClearandInvalidateTimerbyHandle (Variables|Default|GetCharge%20Timer)))

(event EventBeginFiring
  ;[0 1 0.162] Weapon Charging
  ;;[1 1 1] When mouse button is held, begin charging velocity
  (bind _returnvalue (Utilities|Time|SetTimerbyEvent (delegate Custom|Charge%20Weapon) 1.0 true))
  (Variables|Default|SetCharge%20Timer _returnvalue))

(event EventStopFiring
  ;[0 1 0.162] Weapon Charging
  ;;[1 1 1] When released, fire.
  (CallFunction|FireOnce)
  (CallFunction|CancelCharging))

(event EventFireOnce
  ;[1 0 0] Firing weapon
  ;;[1 1 1] Fire weapon if it is not on cooldown, and has been charged enough
  (CallFunction|CancelCharging)
  (if (not (Variables|Default|GetFired%20Recently?))
    (CallFunction|AddtoShots 1)
    ;;[1 1 1] Fire weapon and set it on cooldown
    (Variables|Default|SetFired%20Recently? true)
    (CallFunction|Fire)
    ;;[1 1 1] Set charge to 0, prevent firing until cooldown over
    (Utilities|FlowControl|Sequence
      (:then_0
        (Variables|Charge|SetCharge 0.0))
      (:then_1
        (Utilities|FlowControl|RetriggerableDelay (Variables|Default|GetCooldownTime))
        (Variables|Default|SetFired%20Recently? false)))))

(fn ConstructionScript
  (|CallParentFunction))

(fn Fire
  (CallFunction|PlayCameraShake "/Game/Blueprints/MechSide/BP_Weapons/BP_CameraShake/RailGun.RailGun_C")
  (bind _returnvalue (Game|SpawnActorfromClass "/Game/Blueprints/MechSide/BP_Weapons/BP_Weapons/Projectiles/BP_PitchforkProjectile.BP_PitchforkProjectile_C" (Math|Transform|MakeTransform (Transformation|GetWorldLocation (Variables|Default|GetBarrelSpawn)) (Transformation|GetWorldRotation (Variables|Default|GetCameraUsed))) "Undefined" 0 0))
  (Variables|/Game/Blueprints/MechSide/BP_Weapons/BP_Weapons/Projectiles/BP_PitchforkProjectile.BP_PitchforkProjectile_C|SetOwner%20Gun _returnvalue self)
  (Default|SetVelocitytoCharge _returnvalue (Variables|Charge|GetCharge)))