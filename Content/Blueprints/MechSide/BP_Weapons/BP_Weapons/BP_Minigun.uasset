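; Minigun weapon Blueprint that spins its barrel and fires repeatedly, with tracer and looping-timer driven effects.
; BeginFiring starts slow barrel rotation, then after a short delay speeds it up and calls FireOnce on a timer.
; SpawnProjectileTracer spawns tracers at five barrel points toward the trace end and starts the attached sound once per burst.
; StopFiring halts fire and sound, slowing the barrel briefly before stopping; empty ammo also silences the sound.
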(event Custom|Reset%20Audio
  ;[1 0.7796 0] Spawn a tracer for each barrel location
  (Utilities|FlowControl|DoOnce false) ; enters at Reset
)

(event Custom|Fire
  ;[0.02984 1 0] Begin Firing and Weapon Effect
  (CallFunction|FireOnce))

(event Custom|BeginBarrelMovement
  (bind _barrelpivot (Variables|Default|GetBarrelPivot))
  ;[1 0.3511 0] Start gun slow, then speed up when firing
  (Utilities|FlowControl|Sequence
    (:then_0
      (if (Variables|Default|GetIs%20Firing?)
        (Transformation|AddLocalRotation _barrelpivot "0.000000,0.000000,12.000000" false false)
        (else
          (Transformation|AddLocalRotation _barrelpivot "0.000000,0.000000,4.000000" false false))))
    (:then_1
      (if (<= (Variables|Default|GetCurrentAmmo) 0.0)
        (Utilities|FlowControl|DoOnce false :!label _label
          (:Completed
            (Audio|Components|Audio|Stop (Variables|Default|GetWeaponSound))))
        (else
          (goto _label Reset))))))

(event EventSpawnProjectileTracer
  (params (Location :type Vector :default "0, 0, 0"))
  ;[1 0.7796 0] Spawn a tracer for each barrel location
  (Utilities|FlowControl|Sequence
    (:then_0
      (for _array_element (Utilities|Array|MakeArray (Variables|Default|GetTracerSpawn) (Variables|Default|GetTracerSpawn1) (Variables|Default|GetTracerSpawn2) (Variables|Default|GetTracerSpawn3) (Variables|Default|GetTracerSpawn4))
        (bind _returnvalue (Game|SpawnActorfromClass "/Game/Blueprints/MechSide/BP_Weapons/BP_Weapons/Projectiles/BP_ProjectileTracer.BP_ProjectileTracer_C" (Math|Transform|MakeTransform (Transformation|GetWorldLocation _array_element) (Transformation|GetWorldRotation (Variables|Default|GetCameraUsed))) "Undefined" 0 0))
        (Variables|/Game/Blueprints/MechSide/BP_Weapons/BP_Weapons/Projectiles/BP_ProjectileTracer.BP_ProjectileTracer_C|SetObjectiveLocation%20 _returnvalue (Variables|Default|GetFiringTraceEnd))))
    (:then_1
      (Utilities|FlowControl|DoOnce false
        (:Completed
          (bind _returnvalue_2 (Audio|SpawnSoundAttached "/Game/Sound/Minigun.Minigun" (Variables|Default|GetBarrelSpawn) "None" "0, 0, 0" "0, 0, 0" "KeepRelativeOffset" false 1.0 1.0 0.0 0 0))
          (Variables|Default|SetWeaponSound _returnvalue_2))))))

(event EventBeginFiring
  ;[0.02984 1 0] Begin Firing and Weapon Effect
  (bind _returnvalue (Utilities|Time|SetTimerbyEvent (delegate Custom|BeginBarrelMovement) 0.05 true))
  (bind _output_get (Variables|Default|SetEffectTimer _returnvalue))
  (Utilities|Time|UnpauseTimerbyHandle _output_get)
  (Utilities|FlowControl|Delay 0.5)
  (Variables|Default|SetIs%20Firing? true)
  (bind _returnvalue_2 (Utilities|Time|SetTimerbyEvent (delegate Custom|Fire) 0.1 true))
  (bind _output_get_2 (Variables|Default|SetFireTimer _returnvalue_2))
  (Utilities|Time|UnpauseTimerbyHandle _output_get_2))

(event EventStopFiring
  ;[1 0.06893 0] End firing/ Audio
  (CallFunction|ResetAudio)
  (Audio|Components|Audio|Stop (Variables|Default|GetWeaponSound))
  (Utilities|Time|ClearandInvalidateTimerbyHandle (Variables|Default|GetFireTimer))
  (Variables|Default|SetIs%20Firing? false)
  (Utilities|FlowControl|Delay 0.5)
  (Utilities|Time|ClearandInvalidateTimerbyHandle (Variables|Default|GetEffectTimer)))

(fn ConstructionScript
  (|CallParentFunction))