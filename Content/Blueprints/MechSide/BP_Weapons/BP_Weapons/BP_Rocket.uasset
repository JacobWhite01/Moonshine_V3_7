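; BP_Rocket is a rocket projectile that explodes shortly after its collision overlaps a minion or destructible fence.
; Effect stops the projectile, applies area damage to actors in DetonationSphere, then destroys the rocket.
; Living minions become ragdoll-style physics bodies with an impulse at RocketLaunchPoint, then get stunned or begin their death timer.
; Fences receive heavy damage with a fixed impulse direction.
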(event OnComponentBeginOverlap(Collision)
  (params (OverlappedComponent :type Primitive%20Component%20Object%20Reference) (OtherActor :type Actor%20Object%20Reference) (OtherComp :type Primitive%20Component%20Object%20Reference) (OtherBodyIndex :type Integer) (bFromSweep :type Boolean) (SweepResult :type Hit%20Result%20Structure%20%28by%20ref%29))
  ;[1 1 1] Check if hitting a minion or destructable
  (bind _output_get (Variables|Default|SetInitialised%20Actor OtherActor))
  (if (or (.bSuccess (Utilities|Casting|CastToBP_MinionChar (Variables|Default|GetInitialised%20Actor))) (.bSuccess (Utilities|Casting|CastToBP_DestructibleFence (Variables|Default|GetInitialised%20Actor))))
    (Utilities|FlowControl|Delay 0.2)
    (Effects|SpawnEmitteratLocation "/Game/Assets/ThirdParty/FXVarietyPack/Particles/P_Explosion.P_Explosion" (Transformation|GetActorLocation _output_get) "0, 0, 0" "2.500000,2.500000,2.500000")
    (CallFunction|Effect)))

(fn ConstructionScript)

(fn Effect
  ;[1 1 1] Deal Damage then check if Health is at 0
  (Components|Movement|StopMovementImmediately (Variables|Default|GetProjectileMovement))
  (for _array_element (Collision|GetOverlappingActors (Variables|Default|GetDetonation%20Sphere) "/Script/Engine.Actor" :!class /Script/Engine.PrimitiveComponent)
    (Utilities|FlowControl|Sequence
      (:then_0
        ;[1 1 1] If hit minion isn't below 0 health...
        (bind _asbp_minion_test (Utilities|Casting|CastToBP_MinionChar _array_element))
        (bind _output_get (Variables|Default|SetHitMinion _asbp_minion_test))
        (if (not (<= (Variables|/Game/Blueprints/RobotSide/BP_Minions/BP_MinionChar.BP_MinionChar_C|GetHealth _output_get) 0.0))
          ;[1 1 1] Damage it and apply physics to it
          (Variables|Default|SetOriginal%20location (Transformation|GetActorTransform (Variables|Default|GetHitMinion)))
          (Default|TakeDamage (Variables|Default|GetHitMinion) 5e+01)
          (CallFunction|ApplyPhysicstoMinion)
          (Development|PrintString (Utilities|String|ToString(Float) (Variables|/Game/Blueprints/RobotSide/BP_Minions/BP_MinionChar.BP_MinionChar_C|GetHealth (Variables|Default|GetHitMinion))))
          (if (<= (Variables|/Game/Blueprints/RobotSide/BP_Minions/BP_MinionChar.BP_MinionChar_C|GetHealth (Variables|Default|GetHitMinion)) 0.0)
            (Default|BeginDeathTimer (Variables|Default|GetHitMinion))
            (else
              (Default|StunMinion (Variables|Default|GetHitMinion) self (Variables|Default|GetOriginal%20location))))))
      (:then_1
        ;[1 1 1] Deal damage to destructable meshes
        (bind _asbp_destructible_fence (Utilities|Casting|CastToBP_DestructibleFence _array_element))
        (Default|TakeDamage _asbp_destructible_fence (Transformation|GetActorLocation) (Math|Vector|MakeVector -5e+03 0.0 1e+03) 3e+03))))
  (Actor|DestroyActor))

(fn ApplyPhysicstoMinion
  (bind _hitminion (Variables|Default|GetHitMinion))
  (bind _minionmesh (Variables|/Game/Blueprints/RobotSide/BP_Minions/BP_MinionChar.BP_MinionChar_C|GetMinionMesh _hitminion))
  (bind _rocketlaunchpoint (Variables|/Game/Blueprints/RobotSide/BP_Minions/BP_MinionChar.BP_MinionChar_C|GetRocketLaunchPoint _hitminion))
  (bind _returnvalue (Transformation|GetWorldLocation _rocketlaunchpoint))
  (Collision|SetCollisionEnabled (Variables|/Script/Engine.Character|GetCapsuleComponent (Variables|Default|GetHitMinion)) "NoCollision")
  (Physics|SetSimulatePhysics _minionmesh true)
  (Physics|AddImpulseatLocation _minionmesh (* _returnvalue (Variables|Default|GetRocketImpact)) _returnvalue "None"))