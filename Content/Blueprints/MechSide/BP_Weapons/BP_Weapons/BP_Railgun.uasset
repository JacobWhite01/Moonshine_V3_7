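; Railgun weapon Blueprint that charges while firing is held, then shoots on release above a minimum charge or automatically at full charge.
; A looping timer builds charge, and a cooldown flag blocks rapid refiring.
; FireRailgun traces from the camera, then re-traces from the barrel using only the first result and spawns a laser spline.
; Valid hits trigger an impact effect and charge-scaled minion and overlord damage before charge resets.
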(event Custom|Charge%20Weapon
  ;[1 1 1] Charge weapon and fire if at 100%
  (if (not (Variables|Default|GetFired%20Recently?))
    (if (>= (Variables|Charge|GetCharge) 1e+02)
      (CallFunction|FireOnce)
      (else
        (bind _output_get (Variables|Charge|SetCharge (+ (Variables|Charge|GetCharge) (Variables|Charge|GetCharge%20Increment))))
        (Development|PrintString (Utilities|String|ToString(Float) _output_get))))))

(event Custom|Cancel%20Charging
  ;[1 1 1] Cancel Charging
  (Utilities|Time|ClearandInvalidateTimerbyHandle (Variables|Default|GetChargeTimer)))

(event EventApplyHitEffects
  (params (Hit :type Hit%20Result%20Structure%20%28by%20ref%29))
  (bind (_bblockinghit _binitialoverlap _time _distance _location _impactpoint _normal _impactnormal _physmat _hitactor _hitcomponent _hitbonename) (Collision|BreakHitResult Hit))
  ;[1 1 1] Apply Unique Hit effects
  (CallFunction|AssignHitVariables _impactpoint _hitactor _hitcomponent _hitbonename)
  (if (and _bblockinghit (Utilities|IsValid _hitactor))
    (Utilities|FlowControl|Sequence
      (:then_0
        ;;[1 1 1] Apply Hit then set charge to 0
        (CallFunction|HitEventActor "/Game/Assets/ThirdParty/FXVarietyPack/Particles/P_ky_ThunderBallHit.P_ky_ThunderBallHit"))
      (:then_1
        (CallFunction|HitEventMinion (* (Variables|Charge|GetCharge) (Variables|Default|GetDamage*Minion))))
      (:then_2
        (CallFunction|HitEventOverlord (* (Variables|Default|GetDamage*Overlord) (Variables|Charge|GetCharge)))))))

(event EventBeginFiring
  (bind _returnvalue (Utilities|Time|SetTimerbyEvent (delegate Custom|Charge%20Weapon) 1.0 true))
  (Variables|Default|SetChargeTimer _returnvalue))

(event EventStopFiring
  (CallFunction|FireOnce)
  (CallFunction|CancelCharging))

(event EventFireOnce
  ;[1 1 1] Fire Weapon
  (CallFunction|CancelCharging)
  (if (>= (Variables|Charge|GetCharge) 2e+01)
    (if (not (Variables|Default|GetFired%20Recently?))
      (Variables|Default|SetFired%20Recently? true)
      (bind _outputpin (CallFunction|FireRailgun))
      (Utilities|FlowControl|Sequence
        (:then_0
          (CallFunction|ApplyHitEffects _outputpin)
          (Variables|Charge|SetCharge 0.0)
          (CallFunction|CancelCharging))
        (:then_1
          (Utilities|FlowControl|Delay (Variables|Default|GetCooldownTime))
          (Variables|Default|SetFired%20Recently? false))))))

(fn ConstructionScript
  (|CallParentFunction))

(fn FireRailgun
  (bind _cameraused (Variables|Default|GetCameraUsed))
  (bind _returnvalue (Transformation|GetWorldLocation _cameraused))
  (CallFunction|PlayCameraShake "/Game/Blueprints/MechSide/BP_Weapons/BP_CameraShake/RailGun.RailGun_C")
  (Components|Activation|Activate (Variables|Default|GetMuzzleFlare) false) ; Activate Muzzle flare
  ;[1 1 1] Use Camera Trace for Hit
  (bind _outhits (Collision|MultiLineTraceByChannel _returnvalue (+ _returnvalue (* (Math|Vector|GetForwardVector _cameraused) (Variables|Default|GetRange))) "TraceTypeQuery1" false 0 "None"))
  (for _array_element _outhits
    ;[1 1 1] Use Barrel for particle Trace
    (bind _outhit (Collision|LineTraceByChannel (Transformation|GetWorldLocation (Variables|Default|GetBarrelSpawn)) (.TraceEnd (Collision|BreakHitResult _array_element)) "TraceTypeQuery1" false (Utilities|Array|MakeArray (Variables|Default|GetOwnerActor)) "None"))
    ;[1 1 1] Spawn the laser spline, and designate self as the owner
    (bind _returnvalue_2 (Game|SpawnActorfromClass "/Game/Blueprints/MechSide/BP_Weapons/BP_RailgunSpline.BP_RailgunSpline_C" (Math|Transform|MakeTransform (Transformation|GetWorldLocation (Variables|Default|GetBarrelSpawn)) (Transformation|GetWorldRotation (Variables|Default|GetCameraUsed)) "0.300000,0.300000,0.300000") "Undefined" 0 0))
    (Variables|/Game/Blueprints/MechSide/BP_Weapons/BP_RailgunSpline.BP_RailgunSpline_C|SetWeapon _returnvalue_2 self)
    (Variables|/Game/Blueprints/MechSide/BP_Weapons/BP_RailgunSpline.BP_RailgunSpline_C|SetEnd%20Location _returnvalue_2 (.TraceEnd (Collision|BreakHitResult _array_element)))
    (return _outhit)))