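; Shotgun weapon Blueprint that fires a spread of hitscan pellets from a single trigger event after a short timer delay.
; Each shot checks and decreases ammo, plays sound, camera shake and muzzle flare, then runs randomly offset line traces with projectile tracers.
; Hits spawn impact effects and damage minions, overlords and destructible fences, with damage cut to a quarter beyond a dropoff distance.
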(event EventBeginFiring
  (Utilities|Time|SetTimerbyEvent (delegate EventFireOnce) 0.1))

(event EventFireOnce
  (bind (_start _end) (Utilities|CalculateShotgunSpread -1e+02 1e+02))
  ;[1 1 1] Check if has ammo or firing already
  (bind _has_ammo_ (CallFunction|CheckAmmo 5.0))
  (if _has_ammo_
    (Audio|SpawnSoundAttached "/Game/Sound/Shotgun.Shotgun" (Variables|Default|GetBarrelSpawn) "None" "0, 0, 0" "0, 0, 0" "KeepRelativeOffset" false 1.0 1.0 0.0 0 0)
    (CallFunction|DecreaseAmmo)
    ;[1 1 1] Play Visual Effects
    (CallFunction|PlayCameraShake "/Game/Blueprints/MechSide/BP_Weapons/BP_CameraShake/Shotgun.Shotgun_C")
    (Components|Activation|Activate (Variables|Default|GetMuzzleFlare) false) ; Activate Muzzle flare
    ;[1 1 1] Fire Multiple Shots in Spread
    (for _index (range 0 4)
      (CallFunction|AddtoShots 1)
      (bind _outhit (Collision|LineTraceByChannel _start _end "TraceTypeQuery1" false (Utilities|Array|MakeArray (Variables|Default|GetOwnerActor)) "None"))
      (Variables|Default|SetFiringTraceEnd (.TraceEnd (Collision|BreakHitResult _outhit)))
      (CallFunction|SpawnProjectileTracer (Transformation|GetWorldLocation (Variables|Default|GetBarrelSpawn)))
      (CallFunction|ApplyHitEffects _outhit))))

(event EventApplyHitEffects
  (params (Hit :type Hit%20Result%20Structure%20%28by%20ref%29))
  (bind (_bblockinghit _binitialoverlap _time _distance _location _impactpoint _normal _impactnormal _physmat _hitactor _hitcomponent _hitbonename) (Collision|BreakHitResult Hit))
  (bind (_damge_to_minion _damage_to_overlord _damage_to_destructable) (Utilities|CalculateDropoff _distance))
  ;[1 1 1] Apply Hit Effects
  (CallFunction|AssignHitVariables _impactpoint _hitactor _hitcomponent _hitbonename)
  (if (and _bblockinghit (Utilities|IsValid _hitactor))
    (Utilities|FlowControl|Sequence
      (:then_0
        (CallFunction|HitEventActor "/Game/Assets/Particles/P_BulletImpact.P_BulletImpact"))
      (:then_1
        (CallFunction|HitEventMinion _damge_to_minion))
      (:then_2
        (CallFunction|HitEventOverlord _damage_to_overlord))
      (:then_3
        (bind _asbp_destructible_fence (Utilities|Casting|CastToBP_DestructibleFence (Variables|Default|GetHitActor)))
        (Default|TakeDamage _asbp_destructible_fence (Variables|Default|GetHitLocation) (Variables|Default|GetBullet%20Impact) _damage_to_destructable)))))

(fn ConstructionScript
  (|CallParentFunction))