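; Rocket launcher weapon Blueprint for the mech side that fires a single rocket each time firing begins.
; BeginFiring sets a short one-shot timer to FireOnce, which checks ammo, then plays a camera shake, decrements ammo and activates the muzzle flare.
; It spawns a scaled-up BP_Rocket at the barrel's location, oriented to the camera's rotation rather than the barrel's.
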(event EventBeginFiring
  (Utilities|Time|SetTimerbyEvent (delegate EventFireOnce) 0.1))

(event EventFireOnce
  ;[1 1 1] If not reloading or out of ammo, fire
  (bind _has_ammo_ (CallFunction|CheckAmmo 1.0))
  (if _has_ammo_
    (CallFunction|PlayCameraShake "/Game/Blueprints/MechSide/BP_Weapons/BP_CameraShake/Rocket.Rocket_C")
    (CallFunction|DecreaseAmmo)
    (Components|Activation|Activate (Variables|Default|GetMuzzleFlare) false) ; Activate Muzzle flare
    (Game|SpawnActorfromClass "/Game/Blueprints/MechSide/BP_Weapons/BP_Weapons/BP_Rocket.BP_Rocket_C" (Math|Transform|MakeTransform (Transformation|GetWorldLocation (Variables|Default|GetBarrelSpawn)) (Transformation|GetWorldRotation (Variables|Default|GetCameraUsed)) "2.000000,2.000000,2.000000") "Undefined" 0 0)))

(fn ConstructionScript
  (|CallParentFunction))