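; Gravity well projectile for mech weapons that stuns minions around the point where it detonates.
; Overlaps with anything other than a mech player or another gravity projectile spawn a gravity well particle, then trigger Effect after a short delay.
; Effect stops movement, calls StunMinion on living minions inside DetonationSphere with itself as source, then destroys the projectile.
; The owner is stored through SetupOwnerActor, but the overlap check does not read it.
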(event OnComponentBeginOverlap(CollisionSphere)
  (params (OverlappedComponent :type Primitive%20Component%20Object%20Reference) (OtherActor :type Actor%20Object%20Reference) (OtherComp :type Primitive%20Component%20Object%20Reference) (OtherBodyIndex :type Integer) (bFromSweep :type Boolean) (SweepResult :type Hit%20Result%20Structure%20%28by%20ref%29))
  ;[1 1 1] Check when an actor is hit
  (if (and (!= OtherActor (.AsBP%20Gravity%20Projectile (Utilities|Casting|CastToBP_GravityProjectile OtherActor))) (!= (.AsBP%20Mech%20Player (Utilities|Casting|CastToBP_MechPlayer OtherActor)) OtherActor))
    (Effects|SpawnEmitteratLocation "/Game/Assets/Particles/P_GravityWell.P_GravityWell" (Transformation|GetActorLocation) "0, 0, 0" "0.500000,0.500000,0.500000")
    (Utilities|FlowControl|Delay 0.2)
    (CallFunction|Effect)))

(event Custom|Setup%20Owner%20Actor
  (params (Owner :type Actor%20Object%20Reference))
  ;[1 1 1] Set which mech owns this one (For collision)
  (Variables|Default|SetOwnerActor Owner))

(fn ConstructionScript)

(fn Effect
  ;[1 1 1] Stop projectile movement and begin checking all actors within detonation sphere
  (Components|Movement|StopMovementImmediately (Variables|Default|GetProjectileMovement))
  (for _array_element (Collision|GetOverlappingActors (Variables|Default|GetDetonation%20Sphere) "/Script/Engine.Actor" :!class /Script/Engine.PrimitiveComponent)
    ;[1 1 1] If hit minion isn't below 0 health...
    (bind _asbp_minion_char (Utilities|Casting|CastToBP_MinionChar _array_element))
    (bind _output_get (Variables|Default|SetHitMinion _asbp_minion_char))
    (if (> (Variables|/Game/Blueprints/RobotSide/BP_Minions/BP_MinionChar.BP_MinionChar_C|GetHealth _output_get) 0.0)
      (Default|StunMinion (Variables|Default|GetHitMinion) self (Variables|Default|GetOriginal%20location))))
  (Actor|DestroyActor))