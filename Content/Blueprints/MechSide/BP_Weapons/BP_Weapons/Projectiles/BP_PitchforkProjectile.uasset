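; Pitchfork projectile that damages minions and the Overlord on capsule overlap, then destroys itself.
; A charge event sets its velocity through ConvertVelocity, whose forward-vector scaling math is left unconnected.
; Minion hits deal heavy damage, then ApplyPhysics checks that IsDead is false before stopping movement, disabling capsule collision, ragdolling with a forward impulse and starting the death timer.
; Overlord hits deal lighter damage only.
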(event OnComponentBeginOverlap(CapsuleCollision)
  (params (OverlappedComponent :type Primitive%20Component%20Object%20Reference) (OtherActor :type Actor%20Object%20Reference) (OtherComp :type Primitive%20Component%20Object%20Reference) (OtherBodyIndex :type Integer) (bFromSweep :type Boolean) (SweepResult :type Hit%20Result%20Structure%20%28by%20ref%29))
  ;[1 0 0] Impact Events
  (Utilities|FlowControl|Sequence
    (:then_0
      (bind _asbp_minion_char (Utilities|Casting|CastToBP_MinionChar OtherActor))
      (Default|TakeDamage _asbp_minion_char 1e+02)
      (CallFunction|ApplyPhysics _asbp_minion_char))
    (:then_1
      (bind _asbp_overlord (Utilities|Casting|CastToBP_Overlord OtherActor))
      (Default|TakeDamage _asbp_overlord 2e+01)))
  (Actor|DestroyActor))

(event Custom|Set%20VelocityToCharge
  (params (ChargeMultiplier :type Float%20%28single-precision%29))
  (bind (_end_velocity _projectilemovement) (Utilities|ConvertVelocity ChargeMultiplier))
  ;[1 0.7853 0] Convert player charge to Velocity
  (Variables|/Script/Engine.MovementComponent|SetVelocity _projectilemovement _end_velocity))

(fn ConstructionScript)

(fn ApplyPhysics
  (params (HitMinion :type BP%20Minion%20Char%20Object%20Reference))
  (bind _output_get (LocalVariables|SetMinion HitMinion))
  ;[1 1 1] Apply Physics Effect to Minion if Health at 0
  (if (not (Variables|/Game/Blueprints/RobotSide/BP_Minions/BP_MinionChar.BP_MinionChar_C|GetIsDead? _output_get))
    (Class|NavMovementComponent|StopActiveMovement (Variables|/Script/Engine.Character|GetCharacterMovement (LocalVariables|GetMinion)))
    (Collision|SetCollisionEnabled (Variables|/Script/Engine.Character|GetCapsuleComponent (LocalVariables|GetMinion)) "NoCollision")
    (Physics|SetSimulatePhysics (Variables|/Game/Blueprints/RobotSide/BP_Minions/BP_MinionChar.BP_MinionChar_C|GetMinionMesh (LocalVariables|GetMinion)) true)
    (Physics|AddImpulseatLocation (Variables|/Game/Blueprints/RobotSide/BP_Minions/BP_MinionChar.BP_MinionChar_C|GetMinionMesh (LocalVariables|GetMinion)) (* (Transformation|GetActorForwardVector) 1e+02) "0, 0, 0" "None")
    (Default|BeginDeathTimer (LocalVariables|GetMinion))))