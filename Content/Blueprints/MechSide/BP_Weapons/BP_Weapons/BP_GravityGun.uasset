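; BP_GravityGun is a mech weapon that keeps track of one active gravity projectile and gives its trigger a second function.
; With no projectile in flight, firing starts a short timer, then checks ammo, plays shake and muzzle effects, and spawns an enlarged projectile at the barrel along the camera's rotation.
; Firing again while that projectile exists replaces its velocity with a fast downward drive in its local space.
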(event EventBeginFiring
  ;[1 1 1] When firing check if a projectile is already in flight
  (if (Utilities|IsValid (Variables|Default|GetActive%20Projectile))
    ;[1 1 1] Rotate actors velocity directly downwards
    (Game|Components|ProjectileMovement|SetVelocityinLocalSpace (Variables|/Game/Blueprints/MechSide/BP_Weapons/BP_Weapons/Projectiles/BP_GravityProjectile.BP_GravityProjectile_C|GetProjectileMovement (Variables|Default|GetActive%20Projectile)) "0, 0,-2000.000000")
    (else
      (Utilities|Time|SetTimerbyEvent (delegate EventFireOnce) 0.1))))

(event EventFireOnce
  ;[1 1 1] If not reloading or out of ammo, fire
  (bind _has_ammo_ (CallFunction|CheckAmmo 1.0))
  (if _has_ammo_
    ;[1 1 1] Activate Particles, camera shake etc
    (CallFunction|PlayCameraShake "/Game/Blueprints/MechSide/BP_Weapons/BP_CameraShake/Rocket.Rocket_C")
    (CallFunction|DecreaseAmmo)
    (Components|Activation|Activate (Variables|Default|GetMuzzleFlare) false) ; Activate Muzzle flare
    (bind _returnvalue (Game|SpawnActorfromClass "/Game/Blueprints/MechSide/BP_Weapons/BP_Weapons/Projectiles/BP_GravityProjectile.BP_GravityProjectile_C" (Math|Transform|MakeTransform (Transformation|GetWorldLocation (Variables|Default|GetBarrelSpawn)) (Transformation|GetWorldRotation (Variables|Default|GetCameraUsed)) "2.000000,2.000000,2.000000") "Undefined" 0 0))
    (Variables|Default|SetActive%20Projectile _returnvalue)
    (Default|SetupOwnerActor _returnvalue (Variables|Default|GetOwnerActor))))

(fn ConstructionScript
  (|CallParentFunction))