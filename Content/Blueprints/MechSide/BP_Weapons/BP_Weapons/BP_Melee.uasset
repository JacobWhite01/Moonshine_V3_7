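; Mech melee weapon with constantly spinning blades that damages minions and destructible fences.
; Firing plays a timeline that thrusts the weapon forward, then starts a looping timer running DamageEnemies on actors overlapping the hit box.
; Minions at zero health get physics, an impulse away from the owner and a death timer.
; Stopping fire plays the retract timeline, which clears the damage timer when finished.
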(event Custom|Spin%20Blades
  ;[1 1 1] Spin the Blades each second
  (Transformation|AddLocalRotation (Variables|Default|GetBladePivot) "-40.000000, 0, 0" false false))

(event Custom|Retract%20melee%20weapon
  ;[1 1 1] Attack and Retract Melee weapon
  (bind _backwards_direction (Timeline|Move%20Weapon%20backwards Play)
    (:Update
      (Transformation|AddActorLocalOffset (Math|Vector|MakeVector _backwards_direction 0.0 0.0) false false))
    (:Finished
      (CallFunction|ResetMeleeAnimation)
      (Utilities|Time|ClearandInvalidateTimerbyHandle (Variables|Default|GetMelee_Timer)))))

(event Custom|Reset%20Melee%20Animation
  ;[1 1 1] Attack and Retract Melee weapon
  (Utilities|FlowControl|Sequence
    (:then_0
      (bind _forwards_direction (Timeline|Move%20Weapon%20forwards SetNewTime)
        (:Update
          (Transformation|AddActorLocalOffset (Math|Vector|MakeVector _forwards_direction 0.0 0.0) false false))
        (:Finished
          (bind _returnvalue (Utilities|Time|SetTimerbyFunctionName self "DamageEnemies" 1.0 true))
          (bind _output_get (Variables|Default|SetMelee_Timer _returnvalue))
          (CallFunction|ResetMeleeAnimation)
          (Utilities|Time|UnpauseTimerbyHandle _output_get))))
    (:then_1
      (bind _backwards_direction (Timeline|Move%20Weapon%20backwards SetNewTime)
        (:Update
          (Transformation|AddActorLocalOffset (Math|Vector|MakeVector _backwards_direction 0.0 0.0) false false))
        (:Finished
          (CallFunction|ResetMeleeAnimation)
          (Utilities|Time|ClearandInvalidateTimerbyHandle (Variables|Default|GetMelee_Timer)))))))

(event EventFireOnce
  ;[1 1 1] Attack and Retract Melee weapon
  (bind _forwards_direction (Timeline|Move%20Weapon%20forwards Play)
    (:Update
      (Transformation|AddActorLocalOffset (Math|Vector|MakeVector _forwards_direction 0.0 0.0) false false))
    (:Finished
      (bind _returnvalue (Utilities|Time|SetTimerbyFunctionName self "DamageEnemies" 1.0 true))
      (bind _output_get (Variables|Default|SetMelee_Timer _returnvalue))
      (CallFunction|ResetMeleeAnimation)
      (Utilities|Time|UnpauseTimerbyHandle _output_get))))

(event EventBeginFiring
  (CallFunction|FireOnce))

(event EventBeginPlay
  ;[1 1 1] Spin the Blades each second
  (Utilities|Time|SetTimerbyEvent (delegate Custom|Spin%20Blades) 0.1 true))

(event EventStopFiring
  (CallFunction|RetractMeleeWeapon)
  (CallFunction|ResetMeleeAnimation))

(fn ConstructionScript
  (|CallParentFunction))

(fn DamageEnemies
  (bind _hitminion (Variables|Default|GetHitMinion))
  (bind _minionmesh (Variables|/Game/Blueprints/RobotSide/BP_Minions/BP_MinionChar.BP_MinionChar_C|GetMinionMesh _hitminion))
  ;[1 1 1] Get every actor in Hit box
  (for _array_element (Collision|GetOverlappingActors (Variables|Default|GetHitBox) "/Script/Engine.Actor" :!class /Script/Engine.PrimitiveComponent)
    (Utilities|FlowControl|Sequence
      (:then_0
        ;[1 1 1] All minions in collision radius take damage
        (bind _asbp_minion_char (Utilities|Casting|CastToBP_MinionChar _array_element)
          (:then
            (bind _output_get (Variables|Default|SetHit%20Minion _asbp_minion_char))
            (Default|TakeDamage _output_get 2e+01 (Variables|Default|GetOwnerActor))
            (Components|Activation|Activate (Variables|Default|GetMuzzleFlare) false)
            (if (<= (Variables|/Game/Blueprints/RobotSide/BP_Minions/BP_MinionChar.BP_MinionChar_C|GetHealth _output_get) 0.0)
              ;[1 1 1] Impulse and Destroy minion
              (if (not (Variables|/Game/Blueprints/RobotSide/BP_Minions/BP_MinionChar.BP_MinionChar_C|GetIsDead? (Variables|Default|GetHit%20Minion)))
                (Collision|SetCollisionEnabled (Variables|/Script/Engine.Character|GetCapsuleComponent (Variables|Default|GetHitMinion)) "NoCollision")
                (Physics|SetSimulatePhysics _minionmesh true)
                (Physics|AddImpulseatLocation _minionmesh (* (Math|Rotator|GetRotationXVector (Math|Rotator|FindLookatRotation (Transformation|GetActorLocation (Variables|Default|GetOwnerActor)) (Transformation|GetActorLocation (Variables|Default|GetHit%20Minion)))) (Variables|Default|GetBullet%20Impact)) "0, 0, 0" "None")
                (Default|BeginDeathTimer (Variables|Default|GetHit%20Minion)))))
          (:CastFailed
            (Components|Activation|Deactivate (Variables|Default|GetMuzzleFlare)))))
      (:then_1
        (bind _asbp_destructible_fence (Utilities|Casting|CastToBP_DestructibleFence _array_element))
        (Default|TakeDamage _asbp_destructible_fence (Transformation|GetWorldLocation (Variables|Default|GetBlades)) (Math|Vector|MakeVector -1e+02 0.0 0.0) 1e+03)
        (Components|Activation|Activate (Variables|Default|GetMuzzleFlare) false)))))