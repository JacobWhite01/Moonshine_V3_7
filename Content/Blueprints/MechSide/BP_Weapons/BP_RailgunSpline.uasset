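; Railgun laser beam actor that draws a spline mesh from StartLocation to EndLocation.
; Tick refreshes StartLocation through GetBarrelSpawnPoint, whose barrel lookup on BP_Railgun is unconnected, while EndLocation is never set here.
; A looping timer runs UpdateSpline, which creates one spline mesh if missing and re-stretches it per section, with tangents sampled from the spline and clamped to section length.
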(event Custom|Update%20Spline
  ;[1 1 1] Update all elements of spline mesh
  (Variables|Default|SetSection%20Length (* (.x (Transformation|GetActorScale3D)) 1e+02))
  (for _index (range 0 (Math|Float|Truncate (/ (Spline|GetSplineLength (Variables|Default|GetSpline)) (Variables|Default|GetSection%20Length))))
    ;[1 1 1] If the spline mesh has not been spawned, spawn it
    (if (Utilities|IsValid (Variables|Default|GetSplineMesh))
      _
      (else
        (bind _returnvalue (AddComponent|AddSplineMeshComponent false))
        (bind _output_get (Variables|Default|SetSplineMesh _returnvalue))))
    ;[1 1 1] Update Spline to Match start and end point of laser
    (SplineMesh|SetForwardAxis _output_get "X" true)
    (SplineMesh|SetStartandEnd (Variables|Default|GetSplineMesh) (Variables|Vectors|GetStart%20Location) (Math|Vector|ClampVectorSize (Spline|GetTangentatDistanceAlongSpline (Variables|Default|GetSpline) (* _index (Variables|Default|GetSection%20Length)) "Local") 0.0 (Variables|Default|GetSection%20Length)) (Variables|Vectors|GetEnd%20Location) (Math|Vector|ClampVectorSize (Spline|GetTangentatDistanceAlongSpline (Variables|Default|GetSpline) (* (+ _index 1) (Variables|Default|GetSection%20Length)) "Local") 0.0 (Variables|Default|GetSection%20Length)) true :!class /Script/Engine.SplineMeshComponent)))

(event EventTick
  (params (DeltaSeconds :type Float%20%28single-precision%29))
  ;[1 1 1] Track Players Location
  (Variables|Vectors|SetStart%20Location (Utilities|GetBarrelSpawnPoint)))

(event EventBeginPlay
  (Utilities|Time|SetTimerbyEvent (delegate Custom|Update%20Spline) 0.1 true))

(fn ConstructionScript)